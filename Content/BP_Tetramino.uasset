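; Player-controlled falling tetromino for a Tetris-style game, reused for every piece.
; Tick steps it down on a timer; A/D move and W rotates, reverting when blocked, while S sets the fall interval.
; On landing, it steps back up, has GameManager spawn blocks, resets and respawns itself, then triggers a line check.
; Respawning offsets four cubes into one of five random shapes with random color, column and, where applicable, rotation.
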(event `self.ReceiveBeginPlay`)

(event `self.ReceiveTick`
  (params (DeltaSeconds :type "Float (single-precision)"))
  (`self.GoDown`)
  (if (`self.ColisionWithDown`)
    (`self.K2_AddActorWorldOffset` (0.0 0.0 100.0) :!label _label)
    (`/Game/BP_GameManager.SpawnBlocks` (`self.GameManager`))
    (`self.NormalizeView`)
    (set `self.ColisionWithBlock` false)
    (`/Game/BP_GameManager.CheckLine` (`self.GameManager`))
    (elif (`self.ColisionWithBlock`)
      (goto _label))))

(event `Key|A`
  (params (Key :type "Key Structure"))
  (:`Pressed`
    (`self.GoLeft`)
    (if (`self.ColisionWithBlock`)
      (`self.GoRight`)
      (set `self.ColisionWithBlock` false))))

(event `Key|D`
  (params (Key :type "Key Structure"))
  (:`Pressed`
    (`self.GoRight`)
    (if (`self.ColisionWithBlock`)
      (`self.GoLeft`)
      (set `self.ColisionWithBlock` false))))

(event `Key|W`
  (params (Key :type "Key Structure"))
  (:`Pressed`
    (`self.Rotate`)
    (if (`self.ColisionWithBlock`)
      (`self.Unrotate`)
      (set `self.ColisionWithBlock` false))))

(event `Key|S`
  (params (Key :type "Key Structure"))
  (:`Pressed`
    (set `self.Velocity` 0.1)))

(fn `ContactWithManager`
  (bind _returnvalue (`GameplayStatics.GetActorOfClass` "/Game/BP_GameManager.BP_GameManager_C"))
  (bind _output_get (set `self.GameManager` _returnvalue))
  (set `/Game/BP_GameManager.BP_Tetramino` self _output_get))

(fn `GoDown`
  (bind _output_get (set `self.Timer` (+ (`GameplayStatics.GetWorldDeltaSeconds`) (`self.Timer`))))
  (if (>= _output_get (`self.Velocity`))
    (`self.K2_AddActorWorldOffset` (0.0 0.0 -100.0) true)
    (set `self.Timer` 0.0)))

(fn `GoLeft`
  (`self.K2_AddActorWorldOffset` (0.0 -100.0 0.0) true)
  (if (> (`self.Ylocation`) -400.0)
    (set `self.Ylocation` (- (`self.Ylocation`) 100.0))))

(fn `GoRight`
  (`self.K2_AddActorWorldOffset` (0.0 100.0 0.0) true)
  (if (< (`self.Ylocation`) 400.0)
    (set `self.Ylocation` (+ (`self.Ylocation`) 100.0))))

(fn `NormalizeView`
  (switch `int` (`self.LastViewOfTetramino`)
    (:`0`
      (`SceneComponent.K2_AddLocalOffset` (`self.Cube2`) (0.0 0.0 -100.0) false false)
      (`SceneComponent.K2_AddLocalOffset` (`self.Cube3`) (0.0 0.0 -200.0) false false)
      (`SceneComponent.K2_AddLocalOffset` (`self.Cube4`) (0.0 0.0 -300.0) false false))
    (:`1`
      (`SceneComponent.K2_AddLocalOffset` (`self.Cube2`) (0.0 0.0 -100.0) false false)
      (`SceneComponent.K2_AddLocalOffset` (`self.Cube3`) (0.0 -100.0 -100.0) false false)
      (`SceneComponent.K2_AddLocalOffset` (`self.Cube4`) (0.0 100.0 0.0) false false))
    (:`2`
      (`SceneComponent.K2_AddLocalOffset` (`self.Cube2`) (0.0 100.0 0.0) false false)
      (`SceneComponent.K2_AddLocalOffset` (`self.Cube3`) (0.0 -100.0 0.0) false false)
      (`SceneComponent.K2_AddLocalOffset` (`self.Cube4`) (0.0 0.0 -100.0) false false))
    (:`3`
      (`SceneComponent.K2_AddLocalOffset` (`self.Cube2`) (0.0 100.0 0.0) false false)
      (`SceneComponent.K2_AddLocalOffset` (`self.Cube3`) (0.0 -100.0 0.0) false false)
      (`SceneComponent.K2_AddLocalOffset` (`self.Cube4`) (0.0 100.0 -100.0) false false))
    (:`4`
      (`SceneComponent.K2_AddLocalOffset` (`self.Cube2`) (0.0 -100.0 0.0) false false)
      (`SceneComponent.K2_AddLocalOffset` (`self.Cube3`) (0.0 0.0 -100.0) false false)
      (`SceneComponent.K2_AddLocalOffset` (`self.Cube4`) (0.0 -100.0 -100.0) false false)))
  (`SceneComponent.K2_SetWorldRotation` :`self` (`self.Cube1`))
  (`self.SpawnTetramino`))

(fn `Rotate`
  (bind (_returnvalue_x _returnvalue_y) (`KismetMathLibrary.BreakVector` (`SceneComponent.K2_GetComponentLocation` (`self.Cube1`))))
  (if (`self.NeedRotation`)
    (if (`self.DoubleRotation`)
      (if (`self.FirstRotation`)
        (`self.K2_AddActorWorldRotation` (struct :`Roll` 90.0))
        (`self.K2_AddActorWorldOffset` (0.0 -200.0 0.0) true)
        (set `self.FirstRotation` false)
        (else
          (`self.K2_AddActorWorldRotation` (struct :`Roll` -90.0))
          (`self.K2_AddActorWorldOffset` (`KismetMathLibrary.MakeVector` 0.0 (- (`self.Ylocation`) _returnvalue_y)))
          (set `self.FirstRotation` true)))
      (else
        (`self.K2_AddActorWorldRotation` (struct :`Roll` 90.0))))))

(fn `SetColor`
  (`MaterialInstanceDynamic.SetScalarParameterValue` (`self.Color`) "Color" (`KismetMathLibrary.RandomFloatInRange` 0.0 1.0)))

(fn `SetMaterial`
  (bind _color (`self.Color`))
  (`PrimitiveComponent.SetMaterial` (`self.Cube1`) 0 _color)
  (`PrimitiveComponent.SetMaterial` (`self.Cube2`) 0 _color)
  (`PrimitiveComponent.SetMaterial` (`self.Cube3`) 0 _color)
  (`PrimitiveComponent.SetMaterial` (`self.Cube4`) 0 _color))

(fn `SetRandomViewOfTetramino`
  (bind _output_get (set `self.LastViewOfTetramino` (`KismetMathLibrary.RandomIntegerInRange` 0 4)))
  (switch `int` _output_get
    (:`0`
      (`SceneComponent.K2_AddLocalOffset` (`self.Cube2`) (0.0 0.0 100.0) false false)
      (`SceneComponent.K2_AddLocalOffset` (`self.Cube3`) (0.0 0.0 200.0) false false)
      (`SceneComponent.K2_AddLocalOffset` (`self.Cube4`) (0.0 0.0 300.0) false false)
      (set `self.DoubleRotation` true)
      (bind _output_get_2 (set `self.FirstRotation` (`KismetMathLibrary.RandomBool`)))
      (if (not _output_get_2)
        (`self.K2_AddActorLocalRotation` (struct :`Roll` 90.0))
        (set `self.NeedRotation` true)))
    (:`1`
      (`SceneComponent.K2_AddLocalOffset` (`self.Cube2`) (0.0 0.0 100.0) false false)
      (`SceneComponent.K2_AddLocalOffset` (`self.Cube3`) (0.0 100.0 100.0) false false)
      (`SceneComponent.K2_AddLocalOffset` (`self.Cube4`) (0.0 -100.0 0.0) false false)
      (set `self.DoubleRotation` false)
      (`self.K2_AddActorLocalRotation` (`KismetMathLibrary.MakeRotator` (`KismetMathLibrary.Conv_IntToDouble` (* (`KismetMathLibrary.RandomIntegerInRange` 1 4) 90))))
      (set `self.NeedRotation` true))
    (:`2`
      (`SceneComponent.K2_AddLocalOffset` (`self.Cube2`) (0.0 -100.0 0.0) false false)
      (`SceneComponent.K2_AddLocalOffset` (`self.Cube3`) (0.0 100.0 0.0) false false)
      (`SceneComponent.K2_AddLocalOffset` (`self.Cube4`) (0.0 0.0 100.0) false false)
      (set `self.DoubleRotation` false)
      (`self.K2_AddActorLocalRotation` (`KismetMathLibrary.MakeRotator` (`KismetMathLibrary.Conv_IntToDouble` (* (`KismetMathLibrary.RandomIntegerInRange` 1 4) 90))))
      (set `self.NeedRotation` true))
    (:`3`
      (`SceneComponent.K2_AddLocalOffset` (`self.Cube2`) (0.0 -100.0 0.0) false false)
      (`SceneComponent.K2_AddLocalOffset` (`self.Cube3`) (0.0 100.0 0.0) false false)
      (`SceneComponent.K2_AddLocalOffset` (`self.Cube4`) (0.0 -100.0 100.0) false false)
      (set `self.DoubleRotation` false)
      (`self.K2_AddActorLocalRotation` (`KismetMathLibrary.MakeRotator` (`KismetMathLibrary.Conv_IntToDouble` (* (`KismetMathLibrary.RandomIntegerInRange` 1 4) 90))))
      (set `self.NeedRotation` true))
    (:`4`
      (`SceneComponent.K2_AddLocalOffset` (`self.Cube2`) (0.0 100.0 0.0) false false)
      (`SceneComponent.K2_AddLocalOffset` (`self.Cube3`) (0.0 0.0 100.0) false false)
      (`SceneComponent.K2_AddLocalOffset` (`self.Cube4`) (0.0 100.0 100.0) false false)
      (set `self.NeedRotation` false))))

(fn `SpawnTetramino`
  (bind (_returnvalue_x _returnvalue_y) (`KismetMathLibrary.BreakVector` (`self.K2_GetActorLocation`)))
  (`SceneComponent.K2_SetWorldLocation` (`self.Cube1`) (`KismetMathLibrary.MakeVector` (.x (.location (`SceneComponent.K2_GetComponentToWorld` (`/Game/BP_GameManager.Box` (`self.GameManager`))))) (`KismetMathLibrary.Conv_IntToDouble` (* (`KismetMathLibrary.RandomIntegerInRange` -4 4) 100)) (.z (.location (`SceneComponent.K2_GetComponentToWorld` (`/Game/BP_GameManager.Box` (`self.GameManager`)))))) false false)
  (bind _returnvalue (`KismetMaterialLibrary.CreateDynamicMaterialInstance` "/Game/M_Color.M_Color"))
  (set `self.Color` _returnvalue)
  (`self.SetMaterial`)
  (`self.SetColor`)
  (set `self.Ylocation` _returnvalue_y)
  (set `self.Timer` 0.0)
  (`self.SetRandomViewOfTetramino`))

(fn `Unrotate`
  (bind (_returnvalue_x _returnvalue_y) (`KismetMathLibrary.BreakVector` (`SceneComponent.K2_GetComponentLocation` (`self.Cube1`))))
  (if (`self.NeedRotation`)
    (if (`self.DoubleRotation`)
      (if (`self.FirstRotation`)
        (`self.K2_AddActorWorldRotation` (struct :`Roll` 90.0))
        (`self.K2_AddActorWorldOffset` (0.0 -200.0 0.0) true)
        (set `self.FirstRotation` false)
        (else
          (`self.K2_AddActorWorldRotation` (struct :`Roll` -90.0))
          (`self.K2_AddActorWorldOffset` (`KismetMathLibrary.MakeVector` 0.0 (- (`self.Ylocation`) _returnvalue_y)))
          (set `self.FirstRotation` true)))
      (else
        (`self.K2_AddActorWorldRotation` (struct :`Roll` -90.0))))))

(fn `UserConstructionScript`)