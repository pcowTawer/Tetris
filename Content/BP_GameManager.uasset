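; Game manager for a Tetris-style game that also serves as the player's view target.
; Side cubes push the tetramino back by one 100-unit cell on Tick, while a bottom cube's overlaps toggle its down-collision flag.
; SpawnBlocks copies the piece's four cubes into Block actors with matching materials.
; CheckLine scans height bands, destroys rows of nine blocks and drops those above; neither function is called here.
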(event `self.ReceiveBeginPlay`
  (`self.SetupCamera`))

(event `self.ReceiveActorBeginOverlap`
  (params (OtherActor :type "Actor Object Reference")))

(event `self.ReceiveTick`
  (params (DeltaSeconds :type "Float (single-precision)"))
  (if (`PrimitiveComponent.IsOverlappingActor` (`self.Cube1`) (`self.BP_Tetramino`))
    (`self.K2_AddActorWorldOffset` (`self.BP_Tetramino`) (0.0 100.0 0.0) false false))
  (if (`PrimitiveComponent.IsOverlappingActor` (`self.Cube2`) (`self.BP_Tetramino`))
    (`self.K2_AddActorWorldOffset` (`self.BP_Tetramino`) (0.0 -100.0 0.0) false false)))

(event `self.Cube.OnComponentBeginOverlap`
  (params (OverlappedComponent :type "PrimitiveComponent Object Reference") (OtherActor :type "Actor Object Reference") (OtherComp :type "PrimitiveComponent Object Reference") (OtherBodyIndex :type Integer) (bFromSweep :type Boolean) (SweepResult :type "HitResult Structure (by ref)"))
  (bind _asbp_tetramino (cast `/Game/BP_Tetramino` OtherActor))
  (set `/Game/BP_Tetramino.ColisionWithDown` true _asbp_tetramino))

(event `self.Cube.OnComponentEndOverlap`
  (params (OverlappedComponent :type "PrimitiveComponent Object Reference") (OtherActor :type "Actor Object Reference") (OtherComp :type "PrimitiveComponent Object Reference") (OtherBodyIndex :type Integer))
  (bind _asbp_tetramino (cast `/Game/BP_Tetramino` OtherActor))
  (set `/Game/BP_Tetramino.ColisionWithDown` false _asbp_tetramino))

(fn `CheckBorders`)

(fn `CheckLine`
  (for _index (range 4 19)
    (bind _outactors (`GameplayStatics.GetAllActorsOfClass` "/Game/Block.Block_C"))
    (for _array_element _outactors
      (bind _z (.z (`SceneComponent.K2_GetComponentLocation` (`/Game/Block.Cube` _array_element))))
      (bind _returnvalue (* _index 100.0))
      (if (< _z _returnvalue)
        (if (> _z (+ _returnvalue -100.0))
          (`/Engine/EditorBlueprintResources/StandardMacros.IncrementInt` (`self.LineCounter`)))))
    (if (== (`self.LineCounter`) 9)
      (`KismetArrayLibrary.Array_Set` (`self.Shift`) _index true)
      (set `self.LineCounter` 0)
      (bind _outactors_2 (`GameplayStatics.GetAllActorsOfClass` "/Game/Block.Block_C"))
      (for _array_element_2 _outactors_2
        (bind _z_2 (.z (`SceneComponent.K2_GetComponentLocation` (`/Game/Block.Cube` _array_element_2))))
        (bind _returnvalue_2 (* _index 100.0))
        (if (< _z_2 _returnvalue_2)
          (if (> _z_2 (+ _returnvalue_2 -100.0))
            (`self.K2_DestroyActor` _array_element_2))))
      (else
        (set `self.LineCounter` 0))))
  (for _index_2 (range 19)
    (bind _returnvalue_3 (- 18 _index_2))
    (if (`|GetArrayItem` (`self.Shift`) _returnvalue_3)
      (`KismetArrayLibrary.Array_Set` (`self.Shift`) _returnvalue_3)
      (bind _outactors_3 (`GameplayStatics.GetAllActorsOfClass` "/Game/Block.Block_C"))
      (for _array_element_3 _outactors_3
        (if (not (< (.z (`SceneComponent.K2_GetComponentLocation` (`/Game/Block.Cube` _array_element_3))) (* _returnvalue_3 100.0)))
          (`self.K2_AddActorWorldOffset` _array_element_3 (0.0 0.0 -100.0) false false))))))

(fn `SetupCamera`
  (`PlayerController.SetViewTargetWithBlend` (`GameplayStatics.GetPlayerController` 0) self 0.0 "VTBlend_Linear" 0.0 false))

(fn `SpawnBlocks`
  (bind _bp_tetramino (`self.BP_Tetramino`))
  (bind _cube1 (`/Game/BP_Tetramino.Cube1` _bp_tetramino))
  (bind _cube2 (`/Game/BP_Tetramino.Cube2` _bp_tetramino))
  (bind _cube3 (`/Game/BP_Tetramino.Cube3` _bp_tetramino))
  (bind _cube4 (`/Game/BP_Tetramino.Cube4` _bp_tetramino))
  (bind _returnvalue (`|SpawnActorFromClass` "/Game/Block.Block_C" (`SceneComponent.K2_GetComponentToWorld` _cube1) "Undefined" "OverrideRootScale" null null))
  (`PrimitiveComponent.SetMaterial` (`/Game/Block.Cube` _returnvalue) 0 (`PrimitiveComponent.GetMaterial` _cube1 0))
  (bind _returnvalue_2 (`|SpawnActorFromClass` "/Game/Block.Block_C" (`SceneComponent.K2_GetComponentToWorld` _cube2) "Undefined" "OverrideRootScale" null null))
  (`PrimitiveComponent.SetMaterial` (`/Game/Block.Cube` _returnvalue_2) 0 (`PrimitiveComponent.GetMaterial` _cube2 0))
  (bind _returnvalue_3 (`|SpawnActorFromClass` "/Game/Block.Block_C" (`SceneComponent.K2_GetComponentToWorld` _cube3) "Undefined" "OverrideRootScale" null null))
  (`PrimitiveComponent.SetMaterial` (`/Game/Block.Cube` _returnvalue_3) 0 (`PrimitiveComponent.GetMaterial` _cube3 0))
  (bind _returnvalue_4 (`|SpawnActorFromClass` "/Game/Block.Block_C" (`SceneComponent.K2_GetComponentToWorld` _cube4) "Undefined" "OverrideRootScale" null null))
  (`PrimitiveComponent.SetMaterial` (`/Game/Block.Cube` _returnvalue_4) 0 (`PrimitiveComponent.GetMaterial` _cube4 0)))

(fn `UserConstructionScript`)