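; Player-controlled falling Tetris piece built from four cubes that takes one of seven random shapes with a random color.
; Keys move, rotate and speed up the piece, while Tick steps it down on a timer and reverts to the last transform on block collision.
; On landing it either ends the game near the top, or has BP_GameManager spawn blocks and check lines, reusing itself by undoing shape offsets.
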(event `self.ReceiveBeginPlay`
  (if (not (`self.GameOver`))
    (`self.ContactWithManager`)
    (`self.SpawnTetramino`)))

(event `self.ReceiveTick`
  (params (DeltaSeconds :type "Float (single-precision)"))
  (if (not (`self.GameOver`))
    (`self.CheckBlock`)
    (`self.GoDown`)
    (`self.CheckOnRespawn`)))

(event `Key|A`
  (params (Key :type "Key Structure"))
  (:`Pressed`
    (if (not (`self.GameOver`))
      (`self.GoLeft`))))

(event `Key|D`
  (params (Key :type "Key Structure"))
  (:`Pressed`
    (if (not (`self.GameOver`))
      (`self.GoRight`))))

(event `Key|W`
  (params (Key :type "Key Structure"))
  (:`Pressed`
    (if (not (`self.GameOver`))
      (`self.Rotate`))))

(event `Key|S`
  (params (Key :type "Key Structure"))
  (:`Pressed`
    (set `self.TimeForDown` (* (`self.TimeForDown`) 0.1)))
  (:`Released`
    (set `self.TimeForDown` (* (`self.TimeForDown`) 10.0))))

(event `Key|R`
  (params (Key :type "Key Structure"))
  (:`Pressed`
    (bind _outactors (`GameplayStatics.GetAllActorsOfClass` "/Game/Blueprints/Block.Block_C"))
    (for _array_element _outactors
      (`self.K2_DestroyActor` _array_element))
    (`self.NormalizeView`)))

(fn `CheckBlock`
  (if (`self.ColisionWithBlock`)
    (`self.K2_SetActorTransform` (`self.LastTransform`))))

(fn `CheckOnRespawn`
  (bind (_returnvalue_x _returnvalue_y _returnvalue_z) (`KismetMathLibrary.BreakVector` (`SceneComponent.K2_GetComponentLocation` (`self.Cube1`))))
  (bind (_returnvalue_x_2 _returnvalue_y_2 _returnvalue_z_2) (`KismetMathLibrary.BreakVector` (`SceneComponent.K2_GetComponentLocation` (`self.Cube2`))))
  (bind (_returnvalue_x_3 _returnvalue_y_3 _returnvalue_z_3) (`KismetMathLibrary.BreakVector` (`SceneComponent.K2_GetComponentLocation` (`self.Cube3`))))
  (bind (_returnvalue_x_4 _returnvalue_y_4 _returnvalue_z_4) (`KismetMathLibrary.BreakVector` (`SceneComponent.K2_GetComponentLocation` (`self.Cube4`))))
  (bind (_returnvalue_x_5 _returnvalue_y_5 _returnvalue_z_5) (`KismetMathLibrary.BreakVector` (`SceneComponent.K2_GetComponentLocation` (`/Game/Blueprints/BP_GameManager.Box` (`self.GameManager`)))))
  (if (`self.ColisionWithDown`)
    (if (> _returnvalue_z (- _returnvalue_z_5 200.0)) :!label _label
      (`/Game/Blueprints/BP_GameManager.Game Over` (`self.GameManager`) :!label _label_2)
      (set `self.GameOver` true)
      (elif (> _returnvalue_z_2 (- _returnvalue_z_5 200.0))
        (goto _label_2)
        (elif (> _returnvalue_z_3 (- _returnvalue_z_5 200.0))
          (goto _label_2)
          (elif (> _returnvalue_z_4 (- _returnvalue_z_5 200.0))
            (goto _label_2)
            (else
              (`self.Respawn`))))))
    (elif (`self.ColisionWithBlock`)
      (goto _label))))

(fn `ContactWithManager`
  (bind _returnvalue (`GameplayStatics.GetActorOfClass` "/Game/Blueprints/BP_GameManager.BP_GameManager_C"))
  (bind _output_get (set `self.GameManager` _returnvalue))
  (set `/Game/Blueprints/BP_GameManager.BP_Tetramino` self _output_get))

(fn `GoDown`
  (bind _output_get (set `self.Timer` (+ (`GameplayStatics.GetWorldDeltaSeconds`) (`self.Timer`))))
  (if (>= _output_get (`self.TimeForDown`))
    (set `self.LastTransform` (`self.GetTransform`))
    (`self.K2_AddActorWorldOffset` (0.0 0.0 -100.0) true)
    (set `self.Timer` 0.0)))

(fn `GoLeft`
  (set `self.LastTransform` (`self.GetTransform`))
  (`self.K2_AddActorWorldOffset` (0.0 -100.0 0.0) true)
  (if (> (`self.Ylocation`) -400.0)
    (set `self.Ylocation` (- (`self.Ylocation`) 100.0))))

(fn `GoRight`
  (set `self.LastTransform` (`self.GetTransform`))
  (`self.K2_AddActorWorldOffset` (0.0 100.0 0.0) true)
  (if (< (`self.Ylocation`) 400.0)
    (set `self.Ylocation` (+ (`self.Ylocation`) 100.0))))

(fn `NormalizeView`
  (switch `int` (`self.LastViewOfTetramino`)
    (:`0`
      (`SceneComponent.K2_AddLocalOffset` (`self.Cube2`) (0.0 0.0 100.0) false false)
      (`SceneComponent.K2_AddLocalOffset` (`self.Cube3`) (0.0 0.0 -100.0) false false)
      (`SceneComponent.K2_AddLocalOffset` (`self.Cube4`) (0.0 0.0 -200.0) false false))
    (:`1`
      (`SceneComponent.K2_AddLocalOffset` (`self.Cube2`) (0.0 0.0 -100.0) false false)
      (`SceneComponent.K2_AddLocalOffset` (`self.Cube3`) (0.0 -100.0 -100.0) false false)
      (`SceneComponent.K2_AddLocalOffset` (`self.Cube4`) (0.0 100.0 0.0) false false))
    (:`2`
      (`SceneComponent.K2_AddLocalOffset` (`self.Cube2`) (0.0 100.0 0.0) false false)
      (`SceneComponent.K2_AddLocalOffset` (`self.Cube3`) (0.0 -100.0 0.0) false false)
      (`SceneComponent.K2_AddLocalOffset` (`self.Cube4`) (0.0 0.0 -100.0) false false))
    (:`3`
      (`SceneComponent.K2_AddLocalOffset` (`self.Cube2`) (0.0 100.0 0.0) false false)
      (`SceneComponent.K2_AddLocalOffset` (`self.Cube3`) (0.0 -100.0 0.0) false false)
      (`SceneComponent.K2_AddLocalOffset` (`self.Cube4`) (0.0 100.0 -100.0) false false))
    (:`4`
      (`SceneComponent.K2_AddLocalOffset` (`self.Cube2`) (0.0 -100.0 0.0) false false)
      (`SceneComponent.K2_AddLocalOffset` (`self.Cube3`) (0.0 0.0 -100.0) false false)
      (`SceneComponent.K2_AddLocalOffset` (`self.Cube4`) (0.0 -100.0 -100.0) false false))
    (:`5`
      (`SceneComponent.K2_AddLocalOffset` (`self.Cube2`) (0.0 0.0 -100.0) false false)
      (`SceneComponent.K2_AddLocalOffset` (`self.Cube3`) (0.0 -100.0 0.0) false false)
      (`SceneComponent.K2_AddLocalOffset` (`self.Cube4`) (0.0 100.0 -100.0) false false))
    (:`6`
      (`SceneComponent.K2_AddLocalOffset` (`self.Cube2`) (0.0 100.0 0.0) false false)
      (`SceneComponent.K2_AddLocalOffset` (`self.Cube3`) (0.0 -100.0 0.0) false false)
      (`SceneComponent.K2_AddLocalOffset` (`self.Cube4`) (0.0 -100.0 -100.0) false false)))
  (`SceneComponent.K2_SetWorldRotation` :`self` (`self.Cube1`)))

(fn `Respawn`
  (`self.K2_SetActorTransform` (`self.LastTransform`))
  (`/Game/Blueprints/BP_GameManager.SpawnBlocks` (`self.GameManager`))
  (`self.NormalizeView`)
  (`self.SpawnTetramino`)
  (`/Game/Blueprints/BP_GameManager.CheckLine` (`self.GameManager`)))

(fn `RestartGame`
  (bind _gamemanager (`self.GameManager`))
  (set `self.GameOver` false)
  (set `/Game/Blueprints/BP_GameManager.Score` 0 _gamemanager)
  (`/Game/UI/WBP_Menu.UpdateScore` (`/Game/Blueprints/BP_GameManager.WBP_Menu` _gamemanager))
  (bind _outactors (`GameplayStatics.GetAllActorsOfClass` "/Game/Blueprints/Block.Block_C"))
  (for _array_element _outactors
    (`self.K2_DestroyActor` _array_element))
  (`self.NormalizeView`)
  (`self.SpawnTetramino`))

(fn `Rotate`
  (set `self.LastTransform` (`self.GetTransform`))
  (set `self.isRotate` true)
  (if (`self.NeedRotation`)
    (if (`self.DoubleRotation`)
      (if (`self.FirstRotation`)
        (`self.K2_AddActorWorldRotation` (struct :`Roll` 90.0))
        (set `self.FirstRotation` false)
        (else
          (`self.K2_AddActorWorldRotation` (struct :`Roll` -90.0))
          (set `self.FirstRotation` true)))
      (else
        (`self.K2_AddActorWorldRotation` (struct :`Roll` 90.0))))
    (set `self.isRotate` false)))

(fn `SetColor`
  (`MaterialInstanceDynamic.SetScalarParameterValue` (`self.Color`) "Color" (`KismetMathLibrary.RandomFloatInRange` 0.0 1.0)))

(fn `SetMaterial`
  (bind _color (`self.Color`))
  (`PrimitiveComponent.SetMaterial` (`self.Cube1`) 0 _color)
  (`PrimitiveComponent.SetMaterial` (`self.Cube2`) 0 _color)
  (`PrimitiveComponent.SetMaterial` (`self.Cube3`) 0 _color)
  (`PrimitiveComponent.SetMaterial` (`self.Cube4`) 0 _color))

(fn `SetRandomViewOfTetramino`
  (bind _output_get (set `self.LastViewOfTetramino` (`KismetMathLibrary.RandomIntegerInRange` 0 6)))
  (switch `int` _output_get
    (:`0`
      (`SceneComponent.K2_AddLocalOffset` (`self.Cube2`) (0.0 0.0 -100.0) false false)
      (`SceneComponent.K2_AddLocalOffset` (`self.Cube3`) (0.0 0.0 100.0) false false)
      (`SceneComponent.K2_AddLocalOffset` (`self.Cube4`) (0.0 0.0 200.0) false false)
      (set `self.DoubleRotation` true)
      (set `self.NeedRotation` true)
      (bind _output_get_2 (set `self.FirstRotation` (`KismetMathLibrary.RandomBool`)))
      (if (not _output_get_2)
        (`self.K2_AddActorLocalRotation` (struct :`Roll` 90.0))))
    (:`1`
      (`SceneComponent.K2_AddLocalOffset` (`self.Cube2`) (0.0 0.0 100.0) false false)
      (`SceneComponent.K2_AddLocalOffset` (`self.Cube3`) (0.0 100.0 100.0) false false)
      (`SceneComponent.K2_AddLocalOffset` (`self.Cube4`) (0.0 -100.0 0.0) false false)
      (set `self.DoubleRotation` false)
      (`self.K2_AddActorLocalRotation` (`KismetMathLibrary.MakeRotator` (`KismetMathLibrary.Conv_IntToDouble` (* (`KismetMathLibrary.RandomIntegerInRange` 1 4) 90))))
      (set `self.NeedRotation` true))
    (:`2`
      (`SceneComponent.K2_AddLocalOffset` (`self.Cube2`) (0.0 -100.0 0.0) false false)
      (`SceneComponent.K2_AddLocalOffset` (`self.Cube3`) (0.0 100.0 0.0) false false)
      (`SceneComponent.K2_AddLocalOffset` (`self.Cube4`) (0.0 0.0 100.0) false false)
      (set `self.DoubleRotation` false)
      (`self.K2_AddActorLocalRotation` (`KismetMathLibrary.MakeRotator` (`KismetMathLibrary.Conv_IntToDouble` (* (`KismetMathLibrary.RandomIntegerInRange` 1 4) 90))))
      (set `self.NeedRotation` true))
    (:`3`
      (`SceneComponent.K2_AddLocalOffset` (`self.Cube2`) (0.0 -100.0 0.0) false false)
      (`SceneComponent.K2_AddLocalOffset` (`self.Cube3`) (0.0 100.0 0.0) false false)
      (`SceneComponent.K2_AddLocalOffset` (`self.Cube4`) (0.0 -100.0 100.0) false false)
      (set `self.DoubleRotation` false)
      (`self.K2_AddActorLocalRotation` (`KismetMathLibrary.MakeRotator` (`KismetMathLibrary.Conv_IntToDouble` (* (`KismetMathLibrary.RandomIntegerInRange` 1 4) 90))))
      (set `self.NeedRotation` true))
    (:`4`
      (`SceneComponent.K2_AddLocalOffset` (`self.Cube2`) (0.0 100.0 0.0) false false)
      (`SceneComponent.K2_AddLocalOffset` (`self.Cube3`) (0.0 0.0 100.0) false false)
      (`SceneComponent.K2_AddLocalOffset` (`self.Cube4`) (0.0 100.0 100.0) false false)
      (set `self.NeedRotation` false))
    (:`5`
      (`SceneComponent.K2_AddLocalOffset` (`self.Cube2`) (0.0 0.0 100.0) false false)
      (`SceneComponent.K2_AddLocalOffset` (`self.Cube3`) (0.0 100.0 0.0) false false)
      (`SceneComponent.K2_AddLocalOffset` (`self.Cube4`) (0.0 -100.0 100.0) false false)
      (set `self.DoubleRotation` false)
      (`self.K2_AddActorLocalRotation` (`KismetMathLibrary.MakeRotator` (`KismetMathLibrary.Conv_IntToDouble` (* (`KismetMathLibrary.RandomIntegerInRange` 1 4) 90))))
      (set `self.NeedRotation` true))
    (:`6`
      (`SceneComponent.K2_AddLocalOffset` (`self.Cube2`) (0.0 -100.0 0.0) false false)
      (`SceneComponent.K2_AddLocalOffset` (`self.Cube3`) (0.0 100.0 0.0) false false)
      (`SceneComponent.K2_AddLocalOffset` (`self.Cube4`) (0.0 100.0 100.0) false false)
      (set `self.DoubleRotation` false)
      (`self.K2_AddActorLocalRotation` (`KismetMathLibrary.MakeRotator` (`KismetMathLibrary.Conv_IntToDouble` (* (`KismetMathLibrary.RandomIntegerInRange` 1 4) 90))))
      (set `self.NeedRotation` true))))

(fn `SpawnTetramino`
  (bind (_returnvalue_x _returnvalue_y) (`KismetMathLibrary.BreakVector` (`self.K2_GetActorLocation`)))
  (`SceneComponent.K2_SetWorldLocation` (`self.Cube1`) (`KismetMathLibrary.MakeVector` (.x (.location (`SceneComponent.K2_GetComponentToWorld` (`/Game/Blueprints/BP_GameManager.Box` (`self.GameManager`))))) (`KismetMathLibrary.Conv_IntToDouble` (* (`KismetMathLibrary.RandomIntegerInRange` -4 4) 100)) (.z (.location (`SceneComponent.K2_GetComponentToWorld` (`/Game/Blueprints/BP_GameManager.Box` (`self.GameManager`)))))) false false)
  (bind _returnvalue (`KismetMaterialLibrary.CreateDynamicMaterialInstance` "/Game/Materials/M_Color.M_Color"))
  (set `self.Color` _returnvalue)
  (`self.SetMaterial`)
  (`self.SetColor`)
  (set `self.Ylocation` _returnvalue_y)
  (set `self.Timer` 0.0)
  (`self.SetRandomViewOfTetramino`))

(fn `UserConstructionScript`)