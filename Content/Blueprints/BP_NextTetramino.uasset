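; Next-piece preview actor for a Tetris-style game, showing the upcoming tetromino with four cubes that share one dynamic color material.
; On BeginPlay it creates the material and registers itself with BP_Tetramino.
; ShowNextTetramino stores color, shape and rotation, then calls NormalizeNextTetramino and SetNextTetramino.
; Normalize undoes the LastView shape's relative offsets and resets rotation; Set applies the View shape's offsets, rotation and color.
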(event `self.ReceiveBeginPlay`
  (bind _returnvalue (`KismetMaterialLibrary.CreateDynamicMaterialInstance` "/Game/Materials/M_Color.M_Color"))
  (bind _output_get (set `self.ColorMaterial` _returnvalue))
  (`PrimitiveComponent.SetMaterial` (`self.CubeNextTetramino1`) 0 _output_get)
  (`PrimitiveComponent.SetMaterial` (`self.CubeNextTetramino2`) 0 _output_get)
  (`PrimitiveComponent.SetMaterial` (`self.CubeNextTetramino3`) 0 _output_get)
  (`PrimitiveComponent.SetMaterial` (`self.CubeNextTetramino4`) 0 _output_get)
  (bind _returnvalue_2 (`GameplayStatics.GetActorOfClass` "/Game/Blueprints/BP_Tetramino.BP_Tetramino_C"))
  (set `/Game/Blueprints/BP_Tetramino.BP_NextTetramino` self _returnvalue_2))

(fn `NormalizeNextTetramino`
  (switch `int` (`self.LastView`)
    (:`0`
      (`SceneComponent.K2_AddLocalOffset` (`self.CubeNextTetramino2`) (0.0 0.0 100.0) false false)
      (`SceneComponent.K2_AddLocalOffset` (`self.CubeNextTetramino3`) (0.0 0.0 -100.0) false false)
      (`SceneComponent.K2_AddLocalOffset` (`self.CubeNextTetramino4`) (0.0 0.0 -200.0) false false))
    (:`1`
      (`SceneComponent.K2_AddLocalOffset` (`self.CubeNextTetramino2`) (0.0 0.0 -100.0) false false)
      (`SceneComponent.K2_AddLocalOffset` (`self.CubeNextTetramino3`) (0.0 -100.0 -100.0) false false)
      (`SceneComponent.K2_AddLocalOffset` (`self.CubeNextTetramino4`) (0.0 100.0 0.0) false false))
    (:`2`
      (`SceneComponent.K2_AddLocalOffset` (`self.CubeNextTetramino2`) (0.0 100.0 0.0) false false)
      (`SceneComponent.K2_AddLocalOffset` (`self.CubeNextTetramino3`) (0.0 -100.0 0.0) false false)
      (`SceneComponent.K2_AddLocalOffset` (`self.CubeNextTetramino4`) (0.0 0.0 -100.0) false false))
    (:`3`
      (`SceneComponent.K2_AddLocalOffset` (`self.CubeNextTetramino2`) (0.0 100.0 0.0) false false)
      (`SceneComponent.K2_AddLocalOffset` (`self.CubeNextTetramino3`) (0.0 -100.0 0.0) false false)
      (`SceneComponent.K2_AddLocalOffset` (`self.CubeNextTetramino4`) (0.0 100.0 -100.0) false false))
    (:`4`
      (`SceneComponent.K2_AddLocalOffset` (`self.CubeNextTetramino2`) (0.0 -100.0 0.0) false false)
      (`SceneComponent.K2_AddLocalOffset` (`self.CubeNextTetramino3`) (0.0 0.0 -100.0) false false)
      (`SceneComponent.K2_AddLocalOffset` (`self.CubeNextTetramino4`) (0.0 -100.0 -100.0) false false))
    (:`5`
      (`SceneComponent.K2_AddLocalOffset` (`self.CubeNextTetramino2`) (0.0 0.0 -100.0) false false)
      (`SceneComponent.K2_AddLocalOffset` (`self.CubeNextTetramino3`) (0.0 -100.0 0.0) false false)
      (`SceneComponent.K2_AddLocalOffset` (`self.CubeNextTetramino4`) (0.0 100.0 -100.0) false false))
    (:`6`
      (`SceneComponent.K2_AddLocalOffset` (`self.CubeNextTetramino2`) (0.0 100.0 0.0) false false)
      (`SceneComponent.K2_AddLocalOffset` (`self.CubeNextTetramino3`) (0.0 -100.0 0.0) false false)
      (`SceneComponent.K2_AddLocalOffset` (`self.CubeNextTetramino4`) (0.0 -100.0 -100.0) false false)))
  (`SceneComponent.K2_SetWorldRotation` :`self` (`self.CubeNextTetramino1`)))

(fn `SetNextTetramino`
  (switch `int` (`self.View`)
    (:`0`
      (`SceneComponent.K2_AddLocalOffset` (`self.CubeNextTetramino2`) (0.0 0.0 -100.0) false false)
      (`SceneComponent.K2_AddLocalOffset` (`self.CubeNextTetramino3`) (0.0 0.0 100.0) false false)
      (`SceneComponent.K2_AddLocalOffset` (`self.CubeNextTetramino4`) (0.0 0.0 200.0) false false))
    (:`1`
      (`SceneComponent.K2_AddLocalOffset` (`self.CubeNextTetramino2`) (0.0 0.0 100.0) false false)
      (`SceneComponent.K2_AddLocalOffset` (`self.CubeNextTetramino3`) (0.0 100.0 100.0) false false)
      (`SceneComponent.K2_AddLocalOffset` (`self.CubeNextTetramino4`) (0.0 -100.0 0.0) false false))
    (:`2`
      (`SceneComponent.K2_AddLocalOffset` (`self.CubeNextTetramino2`) (0.0 -100.0 0.0) false false)
      (`SceneComponent.K2_AddLocalOffset` (`self.CubeNextTetramino3`) (0.0 100.0 0.0) false false)
      (`SceneComponent.K2_AddLocalOffset` (`self.CubeNextTetramino4`) (0.0 0.0 100.0) false false))
    (:`3`
      (`SceneComponent.K2_AddLocalOffset` (`self.CubeNextTetramino2`) (0.0 -100.0 0.0) false false)
      (`SceneComponent.K2_AddLocalOffset` (`self.CubeNextTetramino3`) (0.0 100.0 0.0) false false)
      (`SceneComponent.K2_AddLocalOffset` (`self.CubeNextTetramino4`) (0.0 -100.0 100.0) false false))
    (:`4`
      (`SceneComponent.K2_AddLocalOffset` (`self.CubeNextTetramino2`) (0.0 100.0 0.0) false false)
      (`SceneComponent.K2_AddLocalOffset` (`self.CubeNextTetramino3`) (0.0 0.0 100.0) false false)
      (`SceneComponent.K2_AddLocalOffset` (`self.CubeNextTetramino4`) (0.0 100.0 100.0) false false))
    (:`5`
      (`SceneComponent.K2_AddLocalOffset` (`self.CubeNextTetramino2`) (0.0 0.0 100.0) false false)
      (`SceneComponent.K2_AddLocalOffset` (`self.CubeNextTetramino3`) (0.0 100.0 0.0) false false)
      (`SceneComponent.K2_AddLocalOffset` (`self.CubeNextTetramino4`) (0.0 -100.0 100.0) false false))
    (:`6`
      (`SceneComponent.K2_AddLocalOffset` (`self.CubeNextTetramino2`) (0.0 -100.0 0.0) false false)
      (`SceneComponent.K2_AddLocalOffset` (`self.CubeNextTetramino3`) (0.0 100.0 0.0) false false)
      (`SceneComponent.K2_AddLocalOffset` (`self.CubeNextTetramino4`) (0.0 100.0 100.0) false false)))
  (`SceneComponent.K2_AddWorldRotation` (`self.CubeNextTetramino1`) (`KismetMathLibrary.MakeRotator` (`self.AddRotation`)) false false)
  (`MaterialInstanceDynamic.SetScalarParameterValue` (`self.ColorMaterial`) "Color" (`self.Color`)))

(fn `ShowNextTetramino`
  (params (Color :type "Float (double-precision)") (View :type Integer) (AddRotation :type "Float (double-precision)"))
  (set `self.Color` Color)
  (set `self.LastView` (`self.View`))
  (set `self.View` View)
  (set `self.AddRotation` AddRotation)
  (`self.NormalizeNextTetramino`)
  (`self.SetNextTetramino`))

(fn `UserConstructionScript`)